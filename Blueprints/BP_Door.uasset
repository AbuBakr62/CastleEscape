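; BP_Door is an interactable door that a player opens and closes when holding the key for its KeyChannel.
; OnInteraction validates the player, checks HasKey, then toggles between Open and Close based on the Open flag.
; Both events drive one timeline, played forward or reversed, that sets the Door's relative yaw.
; The "Find Key To Open Door!" message prints after closing, while a missing key gives no feedback.
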(event `/Game/Blueprints/InteractableInterface.OnInteraction`
  (params (Player :type "/Game/FirstPersonBP/Blueprints/FirstPersonCharacter Object Reference"))
  (`/Engine/EditorBlueprintResources/StandardMacros.IsValid` Player
    (:`Is Valid`
      (if (`/Game/FirstPersonBP/Blueprints/FirstPersonCharacter.HasKey?` Player (`self.KeyChannel`))
        (if (`self.Open?`)
          (`self.Close`)
          (`KismetSystemLibrary.PrintString` "Find Key To Open Door!")
          (else
            (`self.Open`)))))))

(event `Open`
  (set `self.Open?` true)
  (bind (_direction _doorroatation) (`Timeline|RotateDoorTimeline` :!label _label)
    (:`Update`
      (`SceneComponent.K2_SetRelativeRotation` (`self.Door`) (`KismetMathLibrary.MakeRotator` 0.0 0.0 _doorroatation) false false))))

(event `Close`
  (set `self.Open?` false)
  (goto _label :!via `Reverse`))

(fn `UserConstructionScript`)